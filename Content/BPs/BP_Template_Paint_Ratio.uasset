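; Template Blueprint that periodically measures the paint color ratio of a drawing render target through its ACPaintRatio component and prints it.
; BeginPlay assigns CRT_Drawing to the component and starts a looping two-second timer.
; Each tick records the painted pixels, waits a second as the required gap before reading, then requests the ratio, which returns through a delegate.
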(event Custom|Timer_Read_Ratio
  (Class|ACPaintRatio|RecordPaintedPixels (Variables|Default|GetAC_Paint_Ratio) (Math|Color|MakeColor 255 255 255 255))
  (Utilities|FlowControl|Delay 1.0 :!pinned true) ; There should be atleast 1 second delay between "Record" and "Get Ratio" functions.
  (Class|ACPaintRatio|GetColorRatio (Variables|Default|GetAC_Paint_Ratio) (delegate Custom|Delegate_Ratio) (Math|Color|MakeColor 255 255 255 255)))

(event Custom|Delegate_Ratio
  (params (OutRatio :type Float%20%28double-precision%29))
  (Development|PrintString (Utilities|String|ToString(Float) OutRatio)))

(event EventBeginPlay
  (Variables|/Script/Paint_Ratio.AC_Paint_Ratio|SetCRT_Drawing (Variables|Default|GetAC_Paint_Ratio) "/Paint_Ratio/Textures/CRT_Drawing.CRT_Drawing")
  (Utilities|Time|SetTimerbyEvent (delegate Custom|Timer_Read_Ratio) 2.0 true))

(fn ConstructionScript)